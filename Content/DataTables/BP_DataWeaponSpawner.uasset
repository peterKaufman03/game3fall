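; BP_DataWeaponSpawner is a trigger actor that spawns a random data-driven weapon when the third-person character overlaps its collision.
; It picks a random row from DT_Weapons and spawns a BP_DataWeapon at the Sphere component's location.
; The row's weapon type, elemental type and base damage (as minimum damage) are copied onto the weapon, which then randomizes its data.
; Older text-setting nodes remain unconnected.
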(event OnComponentBeginOverlap(Collision)
  (params (OverlappedComponent :type Primitive%20Component%20Object%20Reference) (OtherActor :type Actor%20Object%20Reference) (OtherComp :type Primitive%20Component%20Object%20Reference) (OtherBodyIndex :type Integer) (bFromSweep :type Boolean) (SweepResult :type Hit%20Result%20Structure%20%28by%20ref%29))
  (Utilities|Casting|CastToBP_ThirdPersonCharacter OtherActor)
  (CallFunction|SpawnWeapon))

(event Custom|SpawnWeapon
  (bind _outrownames (DataTable|GetDataTableRowNames "/Game/DataTables/DT_Weapons.DT_Weapons"))
  (bind _returnvalue (Utilities|GetDataTableRow "/Game/DataTables/DT_Weapons.DT_Weapons" (.OutItem (Utilities|Array|Random _outrownames)))
    (:then
      (bind _returnvalue_2 (Game|SpawnActorfromClass "/Game/DataTables/BP_DataWeapon.BP_DataWeapon_C" (Math|Transform|MakeTransform (Transformation|GetWorldLocation (Variables|Default|GetSphere)) "0, 0, 0" "1.000000,1.000000,1.000000") "Undefined" "MultiplyWithRoot" 0 0))
      (Variables|/Game/DataTables/BP_DataWeapon.BP_DataWeapon_C|SetWeaponType _returnvalue_2 (.weapontypes _returnvalue))
      (Variables|/Game/DataTables/BP_DataWeapon.BP_DataWeapon_C|SetElementalType _returnvalue_2 (.elementaltypes _returnvalue))
      (Variables|/Game/DataTables/BP_DataWeapon.BP_DataWeapon_C|SetMinDamage _returnvalue_2 (.basedamage _returnvalue))
      (Default|RandomizeData _returnvalue_2))))

(fn ConstructionScript)