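; BP_DataWeapon is a weapon actor that displays its type, element and damage range through a mesh, a material and text.
; Weapon and elemental type enums index into mesh and material arrays to set the look of the body.
; RandomizeData nudges minimum damage up, derives maximum damage a random step above it, then refreshes the text, mesh and material.
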(event Custom|RandomizeData
  (bind _output_get (Variables|Default|SetMinDamage (+ (Variables|Default|GetMinDamage) (Math|Random|RandomInteger 2))))
  (Variables|Default|SetMaxDamage (+ _output_get (Math|Random|RandomIntegerinRange 1 4)))
  (CallFunction|UpdateText)
  (CallFunction|SetWeaponMesh)
  (CallFunction|SetWeaponMaterial))

(event Custom|UpdateText
  (Rendering|Components|TextRender|SetText (Variables|Default|GetTextWeaponType) (Utilities|Text|ToText(String) (Utilities|String|EnumtoString (Variables|Default|GetWeaponType))))
  (Rendering|Components|TextRender|SetText (Variables|Default|GetTextElemType) (Utilities|Text|ToText(String) (Utilities|String|EnumtoString (Variables|Default|GetElementalType))))
  (Rendering|Components|TextRender|SetText (Variables|Default|GetTextDamage) (Utilities|Text|ToText(String) (Utilities|String|Append (Utilities|String|ToString(Integer) (Variables|Default|GetMinDamage)) "- " (Utilities|String|ToString(Integer) (Variables|Default|GetMaxDamage))))))

(event Custom|SetWeaponMesh
  (Components|StaticMesh|SetStaticMesh (Variables|Default|GetWeaponBody) (Utilities|Array|Get(acopy) (Variables|Default|GetWeaponMeshes) (Math|Conversions|ToInteger(Byte) (Variables|Default|GetWeaponType)))))

(event Custom|SetWeaponMaterial
  (Rendering|Material|SetMaterial (Variables|Default|GetWeaponBody) 0 (Utilities|Array|Get(acopy) (Variables|Default|GetWeaponMaterials) (Math|Conversions|ToInteger(Byte) (Variables|Default|GetElementalType)))))

(fn ConstructionScript)