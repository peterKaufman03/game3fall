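; BP_SprintPickup is a pickup that grants the player sprinting.
; When BP_ThirdPersonCharacter overlaps its collision, it enables CanSprint and sets Stamina to 10.
; It then records itself in the GM_Game2CoinsSave game mode's LevelSave sprint pickup list and destroys itself.
; A separate CollectedMaterial event swaps the cylinder's material to DiscMaterial.
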(event OnComponentBeginOverlap(collision)
  (params (OverlappedComponent :type Primitive%20Component%20Object%20Reference) (OtherActor :type Actor%20Object%20Reference) (OtherComp :type Primitive%20Component%20Object%20Reference) (OtherBodyIndex :type Integer) (bFromSweep :type Boolean) (SweepResult :type Hit%20Result%20Structure%20%28by%20ref%29))
  (bind _asbp_third_person_character (Utilities|Casting|CastToBP_ThirdPersonCharacter OtherActor))
  (Variables|/Game/ThirdPerson/Blueprints/BP_ThirdPersonCharacter.BP_ThirdPersonCharacter_C|SetCanSprint _asbp_third_person_character true)
  (Variables|/Game/ThirdPerson/Blueprints/BP_ThirdPersonCharacter.BP_ThirdPersonCharacter_C|SetStamina _asbp_third_person_character 1e+01) ; If Stamina is already enabled,\nthis will set stamina to 10.
  (bind _asgm_game_2coins_save (Utilities|Casting|CastToGM_Game2CoinsSave (Game|GetGameMode)))
  (Utilities|Array|AddUnique (Variables|/Game/Save_Load/SG_LevelSave.SG_LevelSave_C|GetSprintPickUPs (Variables|/Game/Save_Load/GM_Game2CoinsSave.GM_Game2CoinsSave_C|GetLevelSave _asgm_game_2coins_save)) self)
  (Actor|DestroyActor))

(event Custom|CollectedMaterial
  (Rendering|Material|SetMaterial (Variables|Default|GetCylinder) 0 "/Engine/VREditor/UI/DiscMaterial.DiscMaterial"))

(fn ConstructionScript)