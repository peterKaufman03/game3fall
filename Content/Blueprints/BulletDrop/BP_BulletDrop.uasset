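; BP_BulletDrop is a debug actor that visualizes bullet drop from its Arrow, comparing a hand-stepped trajectory with Unreal's predicted projectile path.
; BeginPlay loops every half second, drawing the engine prediction, then running BulletDropCalc.
; BulletDropCalc traces segment by segment for SimFrequency steps, dividing only X velocity by frequency and accumulating gravity on Z as per-step displacement.
; It stops at the first blocking hit, then resets position and velocity.
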(event Custom|BulletDropCalc
  (Variables|Default|SetEnd (+ (Variables|Default|GetStartLocation) (/ (Variables|Default|GetVelocity) (Math|Vector|MakeVector (Variables|Default|GetSimFrequency) 1.0 1.0))))
  (Utilities|FlowControl|ForLoopwithBreak 1 (Math|Float|Truncate (Variables|Default|GetSimFrequency)) :!label _label
    (:LoopBody
      (Rendering|Debug|DrawDebugLine (Variables|Default|GetStartLocation) (Variables|Default|GetEnd) "(R=1.000000,G=0.167708,B=0.544583,A=1.000000)" (Variables|Default|GetMaxSimTime) 0.0)
      (Rendering|Debug|DrawDebugSphere (Variables|Default|GetEnd) 5.0 12 "(R=0.091903,G=0.227318,B=1.000000,A=1.000000)" (Variables|Default|GetMaxSimTime))
      (bind _returnvalue (Class|KismetSystemLibrary|LineTraceSinglebyProfile (Variables|Default|GetStartLocation) (Variables|Default|GetEnd) "BlockAll" false 0 "ForDuration" true))
      (if _returnvalue
        (Development|PrintString "Hit Something!" true true "(R=1.000000,G=0.152083,B=0.353989,A=1.000000)")
        (goto _label Break)
        (else
          (Variables|Default|SetStartLocation (Variables|Default|GetEnd))
          (Variables|Default|SetVelocity (+ (Variables|Default|GetVelocity) (Math|Vector|MakeVector 0.0 0.0 (/ -9.8e+02 (Math|Float|Square (Variables|Default|GetSimFrequency))))))
          (Variables|Default|SetEnd (+ (Variables|Default|GetStartLocation) (/ (Variables|Default|GetVelocity) (Math|Vector|MakeVector (Variables|Default|GetSimFrequency) 1.0 1.0)))))))
    (:Completed
      (Variables|Default|SetStartLocation (Transformation|GetWorldLocation (Variables|Default|GetArrow)))
      (Variables|Default|SetVelocity (Variables|Default|GetStartingVelo)))))

(event EventBeginPlay
  (bind _arrow (Variables|Default|GetArrow))
  (bind _returnvalue (Transformation|GetWorldLocation _arrow))
  (Variables|Default|SetStartLocation _returnvalue)
  (Class|GameplayStatics|BlueprintPredictProjectilePathAdvanced (Utilities|Struct|MakePredictProjectilePathParams _returnvalue (Variables|Default|GetStartingVelo) true 0.0 (Variables|Default|GetMaxSimTime) true "ECC_WorldStatic" "ObjectTypeQuery1" 0 (Variables|Default|GetSimFrequency) 0.0 "ForDuration" 1.0 false) :!label _label)
  (Utilities|FlowControl|Delay 0.5)
  (Utilities|FlowControl|Sequence
    (:then_0
      (CallFunction|BulletDropCalc))
    (:then_1
      (goto _label))))

(fn ConstructionScript)