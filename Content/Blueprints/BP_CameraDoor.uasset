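; BP_CameraDoor is a door actor that shows itself opening through a short camera cut.
; OpenDoor, gated on Closed, records the door in the GM_Game2CoinsSave level save, blends the view to itself, then lowers the door mesh by timeline.
; After a pause, it blends back to the supplied view target.
; QuietDoor plays the same movement without camera or save; both paths finish by setting Closed to true.
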(event Custom|OpenDoor
  (params (NewViewTarget :type Actor%20Object%20Reference))
  ;[0.5323 0.1942 0.292] Saves door to the array of open doors in the save game
  (if (Variables|Default|GetClosed)
    (bind _asgm_game_2coins_save (Utilities|Casting|CastToGM_Game2CoinsSave (Game|GetGameMode))
      (:then
        (Utilities|Array|AddUnique (Variables|/Game/Save_Load/SG_LevelSave.SG_LevelSave_C|GetOpenDoors (Variables|/Game/Save_Load/GM_Game2CoinsSave.GM_Game2CoinsSave_C|GetLevelSave _asgm_game_2coins_save)) self))
      (:CastFailed
        _))
    ;[1 1 1] Move Camera to Door Camera
    (Game|Player|SetViewTargetwithBlend (Game|GetPlayerController 0) self (Variables|Default|GetBlend%20Time) "VTBlend_Cubic" 0.0 true)
    (Utilities|FlowControl|Delay (Variables|Default|GetBlend%20Time))
    ;[1 1 1] Open Door
    (bind _newtrack_0 (Timeline|Timeline Play)
      (:Update
        (Transformation|SetRelativeLocation (Variables|Default|GetDoor) (Math|Vector|Lerp(Vector) "0.000000,0.000000,150.000000" "0.000000,0.000000,-130.000000" _newtrack_0) false false))
      (:Finished
        ;[1 1 1] Move Camera Back to Player
        (Utilities|FlowControl|Delay 2.0) ; waiting 2 seconds while the door opens
        (Game|Player|SetViewTargetwithBlend (Game|GetPlayerController 0) NewViewTarget (/ (Variables|Default|GetBlend%20Time) 2.0) "VTBlend_Cubic" 0.0 false) ; shift camera back to player
        (Variables|Default|SetClosed true)))))

(event Custom|QuietDoor
  (bind _newtrack_0 (Timeline|Timeline_0 Play)
    (:Update
      (Transformation|SetRelativeLocation (Variables|Default|GetDoor) (Math|Vector|Lerp(Vector) "0.000000,0.000000,150.000000" "0.000000,0.000000,-130.000000" _newtrack_0) false false))
    (:Finished
      (Variables|Default|SetClosed true))))

(fn ConstructionScript)