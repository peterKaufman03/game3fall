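; Game mode that handles per-level saving of collected coins, sprint pickups, player checkpoint and camera door position, using the level name as save slot.
; BeginPlay loads or creates an SG_LevelSave, reapplies pickups, and restores non-zero player and door transforms, deleting saves that fail the cast.
; CheckPoint and CheckPointDoor store transforms and write to disk.
; FinishLevel clears both transforms before saving, leaving pickup data untouched.
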(event Custom|SaveGame
  (bind _returnvalue (Game|GetCurrentLevelName true))
  (bind _returnvalue_2 (SaveGame|SaveGametoSlot (Variables|Default|GetLevelSave) _returnvalue))
  (if _returnvalue_2
    (Development|PrintString "Level Saved" true true "(R=0.000000,G=0.385417,B=0.139708,A=1.000000)")
    (else
      (Development|PrintString "Level Could Not Be Saved" true true "(R=0.627083,G=0.000000,B=0.071613,A=1.000000)"))))

(event EventBeginPlay
  (bind _returnvalue (Game|GetCurrentLevelName true))
  (bind _returnvalue_2 (SaveGame|DoesSaveGameExist _returnvalue))
  (if _returnvalue_2
    (bind _returnvalue_3 (SaveGame|LoadGamefromSlot _returnvalue))
    (bind _assg_level_save (Utilities|Casting|CastToSG_LevelSave _returnvalue_3)
      (:then
        (bind _output_get (Variables|Default|SetLevelSave _assg_level_save))
        ;[1 0.7965 0.08854] Loading Pickups
        (Default|LoadCollectedCoins _output_get) ; change coins that have been picked up
        (Default|LoadSprintPickUps _output_get)
        ;[1 0.2215 0] Player Location
        (if (not (Class|KismetMathLibrary|EqualExactlyVectorVector (.location (Variables|/Game/Save_Load/SG_LevelSave.SG_LevelSave_C|GetPlayerTransform (Variables|Default|GetLevelSave))) "0, 0, 0"))
          (Transformation|SetWorldTransform (Variables|/Script/Engine.Character|GetCapsuleComponent (Game|GetPlayerCharacter 0)) (Variables|/Game/Save_Load/SG_LevelSave.SG_LevelSave_C|GetPlayerTransform (Variables|Default|GetLevelSave)) false false)
          ;[0.124 0.008393 0.008393] Door State
          (if (Class|KismetMathLibrary|EqualExactlyVectorVector (.location (Variables|/Game/Save_Load/SG_LevelSave.SG_LevelSave_C|GetDoorTransform (Variables|Default|GetLevelSave))) "0, 0, 0")
            (Development|PrintString "Always Zero" true true "(R=0.108095,G=0.121230,B=0.177083,A=1.000000)")
            (else
              (bind _returnvalue_4 (Actor|GetActorOfClass "/Game/Blueprints/BP_CameraDoor.BP_CameraDoor_C"))
              (Transformation|SetWorldTransform (Variables|/Game/Blueprints/BP_CameraDoor.BP_CameraDoor_C|GetDoor _returnvalue_4) (Variables|/Game/Save_Load/SG_LevelSave.SG_LevelSave_C|GetDoorTransform (Variables|Default|GetLevelSave)) false false)))))
      (:CastFailed
        (SaveGame|DeleteGameinSlot _returnvalue)))
    (else
      (bind _returnvalue_5 (SaveGame|CreateSaveGameObject "/Game/Save_Load/SG_LevelSave.SG_LevelSave_C"))
      (Variables|Default|SetLevelSave _returnvalue_5))))

(fn ConstructionScript)

(fn CheckPoint
  (params (PlayerTransform :type Transform))
  (Variables|/Game/Save_Load/SG_LevelSave.SG_LevelSave_C|SetPlayerTransform (Variables|Default|GetLevelSave) PlayerTransform)
  (CallFunction|SaveGame))

(fn FinishLevel
  (Variables|/Game/Save_Load/SG_LevelSave.SG_LevelSave_C|SetPlayerTransform (Variables|Default|GetLevelSave) "")
  (Variables|/Game/Save_Load/SG_LevelSave.SG_LevelSave_C|SetDoorTransform (Variables|Default|GetLevelSave) "")
  (CallFunction|SaveGame))

(fn CheckPointDoor
  (params (DoorTransform :type Transform))
  (Variables|/Game/Save_Load/SG_LevelSave.SG_LevelSave_C|SetDoorTransform (Variables|Default|GetLevelSave) DoorTransform)
  (CallFunction|SaveGame))