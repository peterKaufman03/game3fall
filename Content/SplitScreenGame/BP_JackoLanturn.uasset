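; Jack-o'-lantern pickup that counts down the pumpkins left when collected by a third-person character.
; On BeginPlay it starts a DCS_Piston camera shake from its CameraShakeSource on player controller 0 only.
; When the character overlaps its Collision, it decrements PumpkinsLeft on BP_ThirdPersonGameMode, adds a new W_Collectable widget to the viewport and destroys itself.
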(event OnComponentBeginOverlap(Collision)
  (params (OverlappedComponent :type Primitive%20Component%20Object%20Reference) (OtherActor :type Actor%20Object%20Reference) (OtherComp :type Primitive%20Component%20Object%20Reference) (OtherBodyIndex :type Integer) (bFromSweep :type Boolean) (SweepResult :type Hit%20Result%20Structure%20%28by%20ref%29))
  (Utilities|Casting|CastToBP_ThirdPersonCharacter OtherActor)
  (bind _asbp_third_person_game_mode (Utilities|Casting|CastToBP_ThirdPersonGameMode (Game|GetGameMode)))
  (bind _result (Math|Integer|DecrementInt (Variables|/Game/ThirdPerson/Blueprints/BP_ThirdPersonGameMode.BP_ThirdPersonGameMode_C|GetPumpkinsLeft _asbp_third_person_game_mode))
    (:%20%20
      (Variables|/Game/ThirdPerson/Blueprints/BP_ThirdPersonGameMode.BP_ThirdPersonGameMode_C|SetPumpkinsLeft _asbp_third_person_game_mode _result)
      (bind _returnvalue (UserInterface|CreateWidget "/Game/SplitScreenGame/W_Collectable.W_Collectable_C"))
      (UserInterface|Viewport|AddtoViewport _returnvalue 0)
      (Actor|DestroyActor))))

(event EventBeginPlay
  (Class|PlayerController|ClientStartCameraShakefromSource (Game|GetPlayerController 0) "/Game/Blueprints/CameraShakes/DCS_Piston.DCS_Piston_C" (Variables|Default|GetCameraShakeSource)))

(fn ConstructionScript)