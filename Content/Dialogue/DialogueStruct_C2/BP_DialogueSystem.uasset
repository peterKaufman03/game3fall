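; Dialogue actor that shows lines from DT_TextDialogue when the player presses E inside its collision volume.
; Overlap enables input and shows a next-dialogue prompt; E adds the dialogue widget once and displays the current row, whose index advances after a delay.
; Each row sets the text and maps its character to a material vector parameter, apparently a portrait offset.
; BeginPlay pre-fills the widget through a debug event; a missing row removes it.
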(event OnComponentBeginOverlap(Collision)
  (params (OverlappedComponent :type Primitive%20Component%20Object%20Reference) (OtherActor :type Actor%20Object%20Reference) (OtherComp :type Primitive%20Component%20Object%20Reference) (OtherBodyIndex :type Integer) (bFromSweep :type Boolean) (SweepResult :type Hit%20Result%20Structure%20%28by%20ref%29))
  (Utilities|Casting|CastToBP_ThirdPersonCharacter OtherActor)
  (Input|EnableInput (Game|GetPlayerController 0))
  (bind _returnvalue (UserInterface|CreateWidget "/Game/Dialogue/DialogueStruct_C2/W_NextDialogue.W_NextDialogue_C"))
  (UserInterface|Viewport|AddtoViewport _returnvalue 0))

(event OnComponentEndOverlap(Collision)
  (params (OverlappedComponent :type Primitive%20Component%20Object%20Reference) (OtherActor :type Actor%20Object%20Reference) (OtherComp :type Primitive%20Component%20Object%20Reference) (OtherBodyIndex :type Integer))
  (Utilities|Casting|CastToBP_ThirdPersonCharacter OtherActor)
  (Input|DisableInput (Game|GetPlayerController 0))
  (Widget|RemovefromParent (stale OnComponentBeginOverlap(Collision) _returnvalue)))

(event Custom|Debug%20System
  (bind _w_dialogue (Variables|Default|GetW_Dialogue))
  (bind _characterimage (Variables|/Game/Dialogue/DialogueStruct_C2/W_CharacterSpeakingDialogue.W_CharacterSpeakingDialogue_C|GetCharacterImage _w_dialogue))
  (Development|PrintString "Starting Debug System" true true "(R=0.262583,G=0.480711,B=1.000000,A=1.000000)")
  (bind _outrownames (DataTable|GetDataTableRowNames "/Game/Dialogue/DialogueStruct_C2/DT_TextDialogue.DT_TextDialogue"))
  (bind _returnvalue (Utilities|GetDataTableRow "/Game/Dialogue/DialogueStruct_C2/DT_TextDialogue.DT_TextDialogue" (Utilities|Array|Get(acopy) _outrownames (Variables|Default|GetRowIndex)))
    (:then
      (Rendering|Components|TextRender|SetText (Variables|/Game/Dialogue/DialogueStruct_C2/W_CharacterSpeakingDialogue.W_CharacterSpeakingDialogue_C|GetDialogueTextBlock _w_dialogue) (.text _returnvalue))
      (bind _returnvalue_2 (Appearance|GetDynamicMaterial _characterimage :!class /Script/UMG.Image))
      (Class|Image|SetBrushfromMaterial _characterimage _returnvalue_2)
      (Rendering|Material|SetVectorParameterValue 0 "None" (Utilities|Struct|MakeLinearColor (.x (Utilities|Select :Index (.character _returnvalue) :NewEnumerator0 "0, 0, 0" :NewEnumerator1 "5.000000,2.000000,0.000000" :NewEnumerator2 "3.000000,2.000000,0.000000" :NewEnumerator3 "0.000000,4.000000,0.000000" :NewEnumerator4 "5.000000,4.000000,0.000000" :NewEnumerator5 "5.000000,0.000000,0.000000")) (.y (Utilities|Select :Index (.character _returnvalue) :NewEnumerator0 "0, 0, 0" :NewEnumerator1 "5.000000,2.000000,0.000000" :NewEnumerator2 "3.000000,2.000000,0.000000" :NewEnumerator3 "0.000000,4.000000,0.000000" :NewEnumerator4 "5.000000,4.000000,0.000000" :NewEnumerator5 "5.000000,0.000000,0.000000")) 0.0 1.0) :!class /Script/Engine.KismetMaterialLibrary)
      (Development|PrintString "Vector Parameter Set" true true "(R=1.000000,G=0.239130,B=0.713845,A=1.000000)")
      (Utilities|FlowControl|Delay 2.0)
      (Math|Integer|IncrementInt (Variables|Default|GetRowIndex)))
    (:RowNotFound
      (Development|PrintString "Row Not Found" true true "(R=1.000000,G=0.128360,B=0.164181,A=1.000000)")
      (Widget|RemovefromParent (Variables|Default|GetW_Dialogue)))))

(event Custom|NextLine
  (bind _w_dialogue (Variables|Default|GetW_Dialogue))
  (bind _characterimage (Variables|/Game/Dialogue/DialogueStruct_C2/W_CharacterSpeakingDialogue.W_CharacterSpeakingDialogue_C|GetCharacterImage _w_dialogue))
  (Utilities|FlowControl|Sequence
    (:then_0
      (Utilities|FlowControl|DoOnce false
        (:Completed
          (UserInterface|Viewport|AddtoViewport (Variables|Default|GetW_Dialogue) 0))))
    (:then_1
      (bind _outrownames (DataTable|GetDataTableRowNames "/Game/Dialogue/DialogueStruct_C2/DT_TextDialogue.DT_TextDialogue"))
      (bind _returnvalue (Utilities|GetDataTableRow "/Game/Dialogue/DialogueStruct_C2/DT_TextDialogue.DT_TextDialogue" (Utilities|Array|Get(acopy) _outrownames (Variables|Default|GetRowIndex)))
        (:then
          (Rendering|Components|TextRender|SetText (Variables|/Game/Dialogue/DialogueStruct_C2/W_CharacterSpeakingDialogue.W_CharacterSpeakingDialogue_C|GetDialogueTextBlock _w_dialogue) (.text _returnvalue))
          (bind _returnvalue_2 (Appearance|GetDynamicMaterial _characterimage :!class /Script/UMG.Image))
          (Class|Image|SetBrushfromMaterial _characterimage _returnvalue_2)
          (Rendering|Material|SetVectorParameterValue 0 "None" (Utilities|Struct|MakeLinearColor (.x (Utilities|Select :Index (.character _returnvalue) :NewEnumerator0 "0, 0, 0" :NewEnumerator1 "5.000000,2.000000,0.000000" :NewEnumerator2 "3.000000,2.000000,0.000000" :NewEnumerator3 "0.000000,4.000000,0.000000" :NewEnumerator4 "5.000000,4.000000,0.000000" :NewEnumerator5 "5.000000,0.000000,0.000000")) (.y (Utilities|Select :Index (.character _returnvalue) :NewEnumerator0 "0, 0, 0" :NewEnumerator1 "5.000000,2.000000,0.000000" :NewEnumerator2 "3.000000,2.000000,0.000000" :NewEnumerator3 "0.000000,4.000000,0.000000" :NewEnumerator4 "5.000000,4.000000,0.000000" :NewEnumerator5 "5.000000,0.000000,0.000000")) 0.0 1.0) :!class /Script/Engine.KismetMaterialLibrary)
          (Development|PrintString "Vector Parameter Set" true true "(R=1.000000,G=0.239130,B=0.713845,A=1.000000)")
          (Utilities|FlowControl|Delay 2.0)
          (Math|Integer|IncrementInt (Variables|Default|GetRowIndex)))
        (:RowNotFound
          (Development|PrintString "Row Not Found" true true "(R=1.000000,G=0.128360,B=0.164181,A=1.000000)")
          (Widget|RemovefromParent (Variables|Default|GetW_Dialogue)))))))

(event Custom|Reset%20Add%20to%20View
  (Utilities|FlowControl|DoOnce false) ; enters at Reset
)

(event EventBeginPlay
  (Utilities|FlowControl|Delay 2.0)
  (bind _returnvalue (UserInterface|CreateWidget "/Game/Dialogue/DialogueStruct_C2/W_CharacterSpeakingDialogue.W_CharacterSpeakingDialogue_C"))
  (Variables|Default|SetW_Dialogue _returnvalue)
  (CallFunction|DebugSystem))

(event Input|KeyboardEvents|E
  (params (Key :type Key%20Structure :default "None"))
  (:Pressed
    (CallFunction|NextLine)))

(fn ConstructionScript)